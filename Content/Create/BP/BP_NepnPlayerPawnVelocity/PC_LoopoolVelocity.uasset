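; Player controller for Loopool that handles shot aiming, shot power and a toggleable game-operation widget.
; While the game instance's Shot flag is off, TurnRate yaws the pawn's SpringArmStick, trying BPC_NeonPlayerPawnBase before BP_NeonPlayerPawnVelocity.
; PowerRate adjusts ShotImpluse on the game instance in successive max and min checks, each adding a tenth of the axis value when in range.
; ShowMenu flip-flops the widget created at BeginPlay, starting with removal.
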(event `self.ReceiveBeginPlay`
  (bind _returnvalue (`|CreateWidget` "/Game/Create/Widget/WJ_GameOperation.WJ_GameOperation_C"))
  (set `self.WJ_GameOperation` _returnvalue))

(event `InputAxis|TurnRate`
  (params (AxisValue :type "Float (single-precision)"))
  (bind _returnvalue (`self.K2_GetPawn`))
  (if (`LoopoolGameInstanceC._shot` (`.AsLoopool Game Instance C` (`self.CallInstance`)))
    _
    (elif (!= AxisValue 0.0)
      (`/Engine/EditorBlueprintResources/StandardMacros.IsValid` _returnvalue
        (:`Is Valid`
          ;[1 1 1] C++で作成したクラスか？
          (bind _asbpc_neon_player_pawn_base (cast `/Game/Create/C++/BPC_NeonPlayerPawnBase` _returnvalue)
            (:`then`
              (`SceneComponent.K2_AddRelativeRotation` (`NeonPlayerPawnBase.SpringArmStick` _asbpc_neon_player_pawn_base) (`KismetMathLibrary.MakeRotator` 0.0 0.0 AxisValue) false false))
            (:`CastFailed`
              (bind _asbp_neon_player_pawn_velocity (cast `/Game/Create/BP/BP_NepnPlayerPawnVelocity/BP_NeonPlayerPawnVelocity` _returnvalue)
                (:`then`
                  (`SceneComponent.K2_AddRelativeRotation` (`/Game/Create/BP/BP_NepnPlayerPawnVelocity/BP_NeonPlayerPawnVelocity.SpringArmStick` _asbp_neon_player_pawn_velocity) (`KismetMathLibrary.MakeRotator` 0.0 0.0 AxisValue) false false))
                (:`CastFailed`
                  (`KismetSystemLibrary.PrintString` "CastFaild" true true (struct :`R` 1.0 :`B` 0.44275 :`A` 1.0)))))))))))

(event `InputAxis|PowerRate`
  (params (AxisValue :type "Float (single-precision)"))
  (bind (_asloopoolinstance _asloopool_game_instance_c) (`self.CallInstance`))
  (bind _asloopool_game_instance_c_2 (cast `LoopoolGameInstanceC` (`GameplayStatics.GetGameInstance`) :!pure true))
  (bind _returnvalue (+ (`LoopoolGameInstanceC._shotImpluse` _asloopool_game_instance_c) (/ AxisValue 10.0)))
  (if (not (`LoopoolGameInstanceC._shot` (`.AsLoopool Game Instance C` (`self.CallInstance`))))
    (`|ExecutionSequence`
      (:`then_0`
        ;[1 1 1] 最大値を超えない用に処理
        (if (<= (`LoopoolGameInstanceC._shotImpluse` _asloopool_game_instance_c) (`self.ImpluseMaxValue`))
          (set `LoopoolGameInstanceC._shotImpluse` _returnvalue _asloopool_game_instance_c)
          (else
            (set `LoopoolGameInstanceC._shotImpluse` (`self.ImpluseMaxValue`) _asloopool_game_instance_c))))
      (:`then_1`
        ;[1 1 1] 最小値より低くならないように設定
        (if (>= (`LoopoolGameInstanceC._shotImpluse` _asloopool_game_instance_c_2) (`self.ImpluseMinValue`))
          (set `LoopoolGameInstanceC._shotImpluse` _returnvalue _asloopool_game_instance_c_2)
          (else
            (set `LoopoolGameInstanceC._shotImpluse` (`self.ImpluseMinValue`) _asloopool_game_instance_c_2)))))))

(event `InputAction|ShowMenu`
  (params (Key :type "Key Structure"))
  (bind _wj_gameoperation (`self.WJ_GameOperation`))
  (:`Pressed`
    (`/Engine/EditorBlueprintResources/StandardMacros.FlipFlop`
      (:`A`
        (`Widget.RemoveFromParent` _wj_gameoperation))
      (:`B`
        (`UserWidget.AddToViewport` _wj_gameoperation 0)))))

(fn `UserConstructionScript`)