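; Neon billiard ball pawn, with mesh and number label set from BallNumber, that the player shoots with its own cue stick.
; ActivePawn/NonActive toggle glow, glass opacity, cue, aim arrow and collision type.
; Shot slides the cue by timeline; its hit applies a horizontal impulse scaled by GameInstance ShotImpluse, with a compensation branch for weaker standalone physics.
; DrawLine scales and tints the arrow by shot power; hits play sounds.
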(event `self.ReceiveBeginPlay`)

(event `self.ReceiveTick`
  (params (DeltaSeconds :type "Float (single-precision)"))
  ;[1 1 1] Tick
)

(event `self.poolBall.OnComponentHit`
  (params (HitComponent :type "PrimitiveComponent Object Reference") (OtherActor :type "Actor Object Reference") (OtherComp :type "PrimitiveComponent Object Reference") (NormalImpulse :type "Vector Structure") (Hit :type "HitResult Structure (by ref)"))
  (bind _returnvalue (`KismetMathLibrary.VSize` Hit_ImpactNormal))
  (bind _shotimpluse (`/Game/Create/BP/Loopoolinstance.ShotImpluse` (`self.CallInstance`)))
  (bind _returnvalue_2 (* Hit_ImpactNormal (* _shotimpluse 25.0)))
  ;[1 1 1] Hit
  ;;[0 0 0] スティックと当たったときの処理
  (if (`ActorComponent.ComponentHasTag` OtherComp "Stick")
    (if (> (- (`KismetMathLibrary.VSize` _returnvalue_2) 1.0) (`/Game/Create/BP/BP_NepnPlayerPawnVelocity/PC_LoopoolVelocity.ImpluseMinValue` (`self.CallPlayerController`)))
      (set `self.Impluse` (`KismetMathLibrary.MakeVector` (.x _returnvalue_2) (.y _returnvalue_2))) ; ショットの強さをそのまま衝撃値にする。
      (else
        (`KismetSystemLibrary.PrintString` "Hello")
        (set `self.Impluse` (`KismetMathLibrary.MakeVector` (.x (* Hit_ImpactNormal (`KismetMathLibrary.Conv_DoubleToVector` (* _shotimpluse 133.0)))) (.y (* Hit_ImpactNormal (`KismetMathLibrary.Conv_DoubleToVector` (* _shotimpluse 133.0)))))) ; スタンドアローンだと何故か弱くなるので調整した値を衝撃値にする。
      ))
    (`PrimitiveComponent.AddImpulse` (`self.poolBall`) (`self.Impluse`) "None" false) ; 衝撃を与える
    (bind _returnvalue_3 (`GameplayStatics.SpawnSoundAtLocation` "/Game/Create/Audio/billiard-shot1.billiard-shot1" (`self.K2_GetActorLocation`) (struct) 1.0 1.0 0.0 null null)) ; Shot音を再生
    (`AudioComponent.SetVolumeMultiplier` _returnvalue_3 (* _returnvalue 1.5)) ; 音量を衝撃の値そのままだとうるさいので/10で設定
    (`SceneComponent.SetVisibility` (`self.CueStick`) false false) ; スティックを見えなくする。
    (`PrimitiveComponent.SetCollisionEnabled` (`self.CueStick`) "NoCollision") ; スティックのコリジョンをOFF
    (else
      ;;[0 0 0] ボールに当たったときの処理
      (if (`ActorComponent.ComponentHasTag` OtherComp "Ball")
        (set `self.BallToHit` true)
        (bind _returnvalue_4 (`GameplayStatics.SpawnSoundAtLocation` "/Game/Create/Audio/billiard-ball1.billiard-ball1" (`self.K2_GetActorLocation`) (struct) 1.0 1.0 0.0 null null)) ; 球のHit音を再生
        (`AudioComponent.SetVolumeMultiplier` _returnvalue_4 _returnvalue) ; 衝撃の強さによって音量を変える
      ))))

(event `ActivePawn`
  (bind _poolball (`self.poolBall`))
  ;[1 1 1] ActivePawn（操作しているボールをわかるようにする。）
  (bind _returnvalue (`PrimitiveComponent.CreateDynamicMaterialInstance` _poolball 0 "/Game/PoolTable/Material/Mat_NeonProps.Mat_NeonProps" "None")) ; 操作しているポーンのマテリアルインスタンスを編集
  (`MaterialInstanceDynamic.SetScalarParameterValue` _returnvalue "Emissive_Multiply" 10.0) ; エミッシブカラー（発光）を強くする
  (bind _returnvalue_2 (`PrimitiveComponent.CreateDynamicMaterialInstance` _poolball 1 "/Game/PoolTable/Material/MI_PoolBall_Glass.MI_PoolBall_Glass" "None")) ; 操作しているポーンのマテリアルインスタンスを編集
  (`MaterialInstanceDynamic.SetScalarParameterValue` _returnvalue_2 "Opacity" 0.5) ; ガラス部分を半透明にする。
  (`SceneComponent.SetVisibility` (`self.CueStick`) true false) ; スティックを見せる
  (`PrimitiveComponent.SetCollisionObjectType` (`self.poolBall`) "ECC_Pawn") ; スティックのみにヒットさせるのでコリジョンのタイプを変更
  (`PrimitiveComponent.SetCollisionEnabled` (`self.CueStick`) "QueryAndPhysics") ; スティックのコリジョンを有効化
  (`SceneComponent.SetVisibility` (`self.Arrow`) true false))

(event `NonActive`
  (bind _poolball (`self.poolBall`))
  ;[1 1 1] NonActive
  (bind _returnvalue (`PrimitiveComponent.CreateDynamicMaterialInstance` _poolball 0 "/Game/PoolTable/Material/Mat_NeonProps.Mat_NeonProps" "None")) ; 操作していないポーンのマテリアルインスタンスを編集
  (`MaterialInstanceDynamic.SetScalarParameterValue` _returnvalue "Emissive_Multiply" 1.0) ; エミッシブカラー（発光）を元に戻す
  (bind _returnvalue_2 (`PrimitiveComponent.CreateDynamicMaterialInstance` _poolball 1 "/Game/PoolTable/Material/MI_PoolBall_Glass.MI_PoolBall_Glass" "None")) ; 操作していないポーンのマテリアルインスタンスを編集
  (`MaterialInstanceDynamic.SetScalarParameterValue` _returnvalue_2 "Opacity" 0.0) ; ガラス部分を透明にする。
  (`SceneComponent.SetVisibility` (`self.CueStick`) false false) ; スティックを見せないようにする。
  (`PrimitiveComponent.SetCollisionObjectType` (`self.poolBall`) "ECC_PhysicsBody") ; スティックにHitさせないためにコリジョンのタイプを変更
  (`PrimitiveComponent.SetCollisionEnabled` (`self.CueStick`) "NoCollision") ; スティックのコリジョンを無効化
  (`SceneComponent.K2_SetRelativeLocation` (`self.CueStick`) (0.0 0.0 0.0) false false) ; 打ち終わった後次のshotでHitしないように位置を初期化
  (set `/Game/Create/BP/Loopoolinstance.ShotImpluse` (`/Game/Create/BP/BP_NepnPlayerPawnVelocity/PC_LoopoolVelocity.ImpluseDefaultValue` (`self.CallPlayerController`)) (`self.CallInstance`))
  (`SceneComponent.SetVisibility` (`self.Arrow`) false false))

(event `Shot`
  ;[1 0.9399 0] Shotイベント
  (set `/Game/Create/BP/Loopoolinstance.Shot` true (`self.CallInstance`))
  (bind (_direction _movex _time) (`Timeline|タイムライン_0` :!via `PlayFromStart`) ; 時間とX軸の位置を設定しているタイムライン
    (:`Update`
      (`SceneComponent.K2_SetRelativeLocation` (`self.CueStick`) (`KismetMathLibrary.MakeVector` (`KismetMathLibrary.Lerp` 0.0 _movex _time)) false false))))

(event `DrawLine`
  (bind _pcloopoolvecocity (`self.CallPlayerController`))
  (bind _arrow (`self.Arrow`))
  (bind _shotimpluse (`/Game/Create/BP/Loopoolinstance.ShotImpluse` (`self.CallInstance`)))
  ;[1 1 1] DrawLine
  (if (`/Game/Create/BP/Loopoolinstance.Shot` (`self.CallInstance`))
    (`SceneComponent.SetVisibility` (`self.Arrow`) false false)
    (else
      (`SceneComponent.SetRelativeScale3D` _arrow (`KismetMathLibrary.MakeVector` (/ _shotimpluse 2.0) 1.0 1.0)) ; ArrowコンポーネントのX軸（正面のベクトルの長さ）を設定
      (`ArrowComponent.SetArrowColor` _arrow (`KismetMathLibrary.LinearColorLerp` (struct :`G` 0.118577 :`B` 1.0 :`A` 1.0) (struct :`R` 1.0 :`B` 0.037502 :`A` 1.0) (`KismetMathLibrary.NormalizeToRange` _shotimpluse (`/Game/Create/BP/BP_NepnPlayerPawnVelocity/PC_LoopoolVelocity.ImpluseMinValue` _pcloopoolvecocity) (`/Game/Create/BP/BP_NepnPlayerPawnVelocity/PC_LoopoolVelocity.ImpluseMaxValue` _pcloopoolvecocity)))) ; Lerpで計算された色をArrowColorに設定
    )))

(event `BL_Init`
  ;[1 1 1] PlayerのショットフラグとHitフラグを初期化
  (set `/Game/Create/BP/Loopoolinstance.Shot` false (`self.CallInstance`))
  (set `self.BallToHit` false))

(event `ShowBallnum`
  (bind _numbertext (`self.numberText`))
  ;[1 1 1] ボールの番号を見せるイベント
  (`/Engine/EditorBlueprintResources/StandardMacros.FlipFlop`
    (:`A`
      (`SceneComponent.SetVisibility` _numbertext true false))
    (:`B`
      (`SceneComponent.SetVisibility` _numbertext false false))))

(event `ShowVelocity`
  ;[1 0 0] (デバッグ用）スピード値を表示
  (`KismetSystemLibrary.PrintString` (`KismetStringLibrary.Concat_StrStr` (`KismetSystemLibrary.GetDisplayName` self) " = " (`KismetStringLibrary.Conv_DoubleToString` (`KismetMathLibrary.VSize` (`self.GetVelocity`))))))

(fn `UserConstructionScript`
  ;[1 1 1] Spawn Compoment And Static Mesh
  (`|ExecutionSequence`
    (:`then_0`
      ;[1 1 1] poolball
      ;;[1 1 1] Main Function
      (`StaticMeshComponent.SetStaticMesh` (`self.poolBall`) (`|GetArrayItem` (`self.Ref-BallMeshes`) (`self.BallNumber`))))
    (:`then_1`
      ;[1 1 1] マテリアル設定
      (bind _returnvalue (`PrimitiveComponent.CreateDynamicMaterialInstance` (`self.poolBall`) 0 "/Game/PoolTable/Material/Mat_NeonProps.Mat_NeonProps" "None"))
      (`MaterialInstanceDynamic.SetScalarParameterValue` _returnvalue "Emissive_Multiply" 1.0)
      (bind _returnvalue_2 (`PrimitiveComponent.CreateDynamicMaterialInstance` (`self.poolBall`) 1 "/Game/PoolTable/Material/MI_PoolBall_Glass.MI_PoolBall_Glass" "None"))
      (`MaterialInstanceDynamic.SetScalarParameterValue` _returnvalue_2 "Opacity" 0.5))
    (:`then_2`
      ;[1 1 1] テキスト設定
      (`TextRenderComponent.K2_SetText` (`self.numberText`) (`KismetTextLibrary.Conv_StringToText` (`KismetStringLibrary.Conv_IntToString` (`self.BallNumber`)))))))