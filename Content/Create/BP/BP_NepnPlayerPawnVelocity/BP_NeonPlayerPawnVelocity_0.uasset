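; Player pawn Blueprint that draws a debug sphere marker on its pool ball while the game instance's Shot flag is false.
; A looping timer started on BeginPlay fires DrawTarget every tenth of a second.
; DrawTarget uses a zero-length sphere object trace against WorldStatic purely for its timed debug drawing, since the hit result is unused.
; Tick is disabled, and an alternative DrawDebugSphere node is left unconnected.
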(event `self.ReceiveBeginPlay`
  (`parent.ReceiveBeginPlay`)
  (`KismetSystemLibrary.K2_SetTimerDelegate` (delegate `DrawTarget`) 0.1 true))

(event `DrawTarget`
  (bind _returnvalue (`SceneComponent.K2_GetComponentLocation` (`self.poolBall`)))
  (if (not (`/Game/Create/BP/Loopoolinstance.Shot` (cast `/Game/Create/BP/Loopoolinstance` (`GameplayStatics.GetGameInstance`) :!pure true)))
    (`KismetSystemLibrary.SphereTraceSingleForObjects` :`Start` _returnvalue :`End` _returnvalue :`Radius` 3.0 :`ObjectTypes` (`|MakeArray` "ObjectTypeQuery1" :!type "EObjectTypeQuery Enum") :`DrawDebugType` "ForDuration" :`TraceHitColor` (struct :`R` 1.0 :`A` 1.0) :`DrawTime` 0.1)))

(fn `UserConstructionScript`
  (`parent.UserConstructionScript`))