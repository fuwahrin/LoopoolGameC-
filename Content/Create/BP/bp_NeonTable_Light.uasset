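; Neon pool table Blueprint that detects pocketed balls, ends the game and plays table impact sounds.
; A "Ball"-tagged component overlapping BollCheckPlate plays a pocket sound and sets the game mode's GameResult true only if its display name ends in "0".
; The result event disables input, shows the result widget, then resets Shot and opens Title after a delay.
; Cushion hits share a function that scales sound volume by impulse, with a cap.
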(event `self.ReceiveBeginPlay`
  (bind _returnvalue (`|CreateWidget` "/Game/Create/Widget/Wj_GameResult.WJ_GameResult_C"))
  (set `self.WJ_GameResutl` _returnvalue))

(event `self.BollCheckPlate.OnComponentBeginOverlap`
  (params (OverlappedComponent :type "PrimitiveComponent Object Reference") (OtherActor :type "Actor Object Reference") (OtherComp :type "PrimitiveComponent Object Reference") (OtherBodyIndex :type Integer) (bFromSweep :type Boolean) (SweepResult :type "HitResult Structure (by ref)"))
  (bind _aspool_velocity_mode (cast `/Game/Create/BP/BP_NepnPlayerPawnVelocity/PoolVelocityMode` (`GameplayStatics.GetGameMode`) :!pure true))
  (if (`ActorComponent.ComponentHasTag` OtherComp "Ball")
    (`GameplayStatics.SpawnSoundAtLocation` "/Game/Create/Audio/billiard-pocket1.billiard-pocket1" (`SceneComponent.K2_GetComponentLocation` OtherComp))
    (if (`KismetStringLibrary.EqualEqual_StrStr` (`KismetStringLibrary.Right` (`KismetSystemLibrary.GetDisplayName` OtherComp) 1) "0")
      (set `/Game/Create/BP/BP_NepnPlayerPawnVelocity/PoolVelocityMode.GameResult` true _aspool_velocity_mode)
      (else
        (set `/Game/Create/BP/BP_NepnPlayerPawnVelocity/PoolVelocityMode.GameResult` false _aspool_velocity_mode)))
    (`self.GameResult_Event`)))

(event `GameResult_Event`
  (`self.DisableInput` (`GameplayStatics.GetPlayerController` 0) null) ; 入力を停止する。
  (`UserWidget.AddToViewport` (`self.WJ_GameResutl`) 0)
  (`KismetSystemLibrary.Delay` 3.0)
  (set `/Game/Create/BP/Loopoolinstance.Shot` false (cast `/Game/Create/BP/Loopoolinstance` (`GameplayStatics.GetGameInstance`) :!pure true))
  (`GameplayStatics.OpenLevel` "Title"))

(event `self.RightDown.OnComponentHit`
  (params (HitComponent :type "PrimitiveComponent Object Reference") (OtherActor :type "Actor Object Reference") (OtherComp :type "PrimitiveComponent Object Reference") (NormalImpulse :type "Vector Structure") (Hit :type "HitResult Structure (by ref)"))
  (`self.SpawnSoundWallHIt` Hit NormalImpulse))

(event `self.RightUp.OnComponentHit`
  (params (HitComponent :type "PrimitiveComponent Object Reference") (OtherActor :type "Actor Object Reference") (OtherComp :type "PrimitiveComponent Object Reference") (NormalImpulse :type "Vector Structure") (Hit :type "HitResult Structure (by ref)"))
  (`self.SpawnSoundWallHIt` Hit NormalImpulse))

(event `self.LeftDown.OnComponentHit`
  (params (HitComponent :type "PrimitiveComponent Object Reference") (OtherActor :type "Actor Object Reference") (OtherComp :type "PrimitiveComponent Object Reference") (NormalImpulse :type "Vector Structure") (Hit :type "HitResult Structure (by ref)"))
  (`self.SpawnSoundWallHIt` Hit NormalImpulse))

(event `self.LeftUp.OnComponentHit`
  (params (HitComponent :type "PrimitiveComponent Object Reference") (OtherActor :type "Actor Object Reference") (OtherComp :type "PrimitiveComponent Object Reference") (NormalImpulse :type "Vector Structure") (Hit :type "HitResult Structure (by ref)"))
  (`self.SpawnSoundWallHIt` Hit NormalImpulse))

(event `self.Bottom.OnComponentHit`
  (params (HitComponent :type "PrimitiveComponent Object Reference") (OtherActor :type "Actor Object Reference") (OtherComp :type "PrimitiveComponent Object Reference") (NormalImpulse :type "Vector Structure") (Hit :type "HitResult Structure (by ref)"))
  (`self.SpawnSoundWallHIt` Hit NormalImpulse))

(event `self.Top.OnComponentHit`
  (params (HitComponent :type "PrimitiveComponent Object Reference") (OtherActor :type "Actor Object Reference") (OtherComp :type "PrimitiveComponent Object Reference") (NormalImpulse :type "Vector Structure") (Hit :type "HitResult Structure (by ref)"))
  (`self.SpawnSoundWallHIt` Hit NormalImpulse))

(event `self.Bottom1.OnComponentHit`
  (params (HitComponent :type "PrimitiveComponent Object Reference") (OtherActor :type "Actor Object Reference") (OtherComp :type "PrimitiveComponent Object Reference") (NormalImpulse :type "Vector Structure") (Hit :type "HitResult Structure (by ref)"))
  (`self.SpawnSoundWallHIt` Hit NormalImpulse))

(event `self.Bottom2.OnComponentHit`
  (params (HitComponent :type "PrimitiveComponent Object Reference") (OtherActor :type "Actor Object Reference") (OtherComp :type "PrimitiveComponent Object Reference") (NormalImpulse :type "Vector Structure") (Hit :type "HitResult Structure (by ref)"))
  (`self.SpawnSoundWallHIt` Hit NormalImpulse))

(event `self.LeftUp1.OnComponentHit`
  (params (HitComponent :type "PrimitiveComponent Object Reference") (OtherActor :type "Actor Object Reference") (OtherComp :type "PrimitiveComponent Object Reference") (NormalImpulse :type "Vector Structure") (Hit :type "HitResult Structure (by ref)"))
  (`self.SpawnSoundWallHIt` Hit NormalImpulse))

(event `self.LeftDown1.OnComponentHit`
  (params (HitComponent :type "PrimitiveComponent Object Reference") (OtherActor :type "Actor Object Reference") (OtherComp :type "PrimitiveComponent Object Reference") (NormalImpulse :type "Vector Structure") (Hit :type "HitResult Structure (by ref)"))
  (`self.SpawnSoundWallHIt` Hit NormalImpulse))

(event `self.RightUp1.OnComponentHit`
  (params (HitComponent :type "PrimitiveComponent Object Reference") (OtherActor :type "Actor Object Reference") (OtherComp :type "PrimitiveComponent Object Reference") (NormalImpulse :type "Vector Structure") (Hit :type "HitResult Structure (by ref)"))
  (`self.SpawnSoundWallHIt` Hit NormalImpulse))

(event `self.RightDown1.OnComponentHit`
  (params (HitComponent :type "PrimitiveComponent Object Reference") (OtherActor :type "Actor Object Reference") (OtherComp :type "PrimitiveComponent Object Reference") (NormalImpulse :type "Vector Structure") (Hit :type "HitResult Structure (by ref)"))
  (`self.SpawnSoundWallHIt` Hit NormalImpulse))

(event `self.Top1.OnComponentHit`
  (params (HitComponent :type "PrimitiveComponent Object Reference") (OtherActor :type "Actor Object Reference") (OtherComp :type "PrimitiveComponent Object Reference") (NormalImpulse :type "Vector Structure") (Hit :type "HitResult Structure (by ref)"))
  (`self.SpawnSoundWallHIt` Hit NormalImpulse))

(event `self.Top2.OnComponentHit`
  (params (HitComponent :type "PrimitiveComponent Object Reference") (OtherActor :type "Actor Object Reference") (OtherComp :type "PrimitiveComponent Object Reference") (NormalImpulse :type "Vector Structure") (Hit :type "HitResult Structure (by ref)"))
  (`self.SpawnSoundWallHIt` Hit NormalImpulse))

(fn `UserConstructionScript`)